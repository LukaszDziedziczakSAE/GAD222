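; Modular zombie character that randomizes its walk speed and outfit, then wanders or chases the player.
; When velocity drops to zero, it waits briefly, then moves to the player or a random reachable point, depending on Chase.
; BPC_OutfitController randomizes the look in construction and optionally at BeginPlay.
; Events gather tagged mesh components to clear dynamic parts, set materials by slot name and apply static morph targets.
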(event Custom|ClearComponents
  ;[0 0.7457 1] Clears Dynamic Components - Prevents unused components from remaining after respawn/initilization
  (CallFunction|SetComponentArrays)
  (Utilities|FlowControl|Sequence
    (:then_0
      (for _array_element (Variables|Default|GetSkeletalMesh)
        (if (not (Components|ComponentHasTag _array_element "UE5Master"))
          (if (Components|ComponentHasTag _array_element "Parent")
            (Components|SkinnedMesh|SetSkinnedAssetandUpdate _array_element 0 true)
            (else
              (Components|DestroyComponent _array_element))))))
    (:then_1
      (for _array_element_2 (Variables|Default|GetStaticMesh)
        (Components|DestroyComponent _array_element_2)))))

(event Custom|SetComponentArrays
  ;[1 0.2964 0] Loads Dynamic Skeletal Mesh Components which are not accessible Via OutfitController component
  (Utilities|Array|Clear (Variables|Default|GetSkeletalMesh))
  (Utilities|Array|Clear (Variables|Default|GetStaticMesh))
  (Utilities|FlowControl|Sequence
    (:then_0
      (Variables|Default|SetSkeletalMesh (Actor|GetComponentsbyTag "/Script/Engine.SkeletalMeshComponent" "OutfitController"))
      (Utilities|Array|Add (Variables|Default|GetSkeletalMesh) (Utilities|Array|Get(acopy) (Actor|GetComponentsbyTag "/Script/Engine.SkeletalMeshComponent" "Parent"))))
    (:then_1
      (Variables|Default|SetStaticMesh (Actor|GetComponentsbyTag "/Script/Engine.StaticMeshComponent" "OutfitController")))))

(event Custom|SetMorphTarget
  (params (RandomValues :type Float%20%28double-precision%29))
  ;[1 0.5974 0.487] Set Morph Target - This is for static morph targets like muscularity etc. These are not animated.
  (CallFunction|SetComponentArrays)
  (for _array_element (Variables|Default|GetSkeletalMesh)
    (bind _array_element_2 (Utilities|Array|ForEachLoopwithBreak (Variables|/Game/YI_ModularZombies/Blueprints/Master/Components/BPC_OutfitController.BPC_OutfitController_C|GetMorphTargets (Variables|Default|GetAs%20BPC%20Outfit%20Controller)))
      (:LoopBody
        (for _array_element_3 (.MorphposeName (Utilities|Struct|BreakStruc_StaticMorphPoses _array_element_2))
          (Components|SkeletalMesh|SetMorphTarget _array_element (Utilities|String|StringToName _array_element_3) RandomValues true))))))

(event Custom|SetMaterials
  (params (SlotNames :type Array%20of%20Strings) (ParameterNames :type Array%20of%20Strings) (Materials :type Array%20of%20Material%20Instance%20Object%20References) (ParameterValue :type Float%20%28double-precision%29) (RandomizeParameters :type Boolean))
  (bind _skeletalmesh (Variables|Default|GetSkeletalMesh))
  ;[0 0 0] Set the Materials based on OutfitController component configuration
  (CallFunction|SetComponentArrays)
  (if RandomizeParameters
    (for (_array_element _array_index) Materials
      (bind _returnvalue (Rendering|Material|CreateDynamicMaterialInstance _array_element "None" "Transient" :!class /Script/Engine.KismetMaterialLibrary))
      (for _array_element_2 ParameterNames
        (Utilities|IsValid _returnvalue
          (:Is%20Valid
            (Rendering|Material|SetScalarParameterValue _returnvalue (Utilities|String|StringToName _array_element_2) ParameterValue :!class /Script/Engine.MaterialInstanceDynamic))))
      (for _array_element_3 _skeletalmesh
        (Rendering|Material|SetMaterialbyName _array_element_3 (Utilities|String|StringToName (Utilities|Array|Get(acopy) SlotNames _array_index)) _returnvalue)))
    (else
      (for (_array_element_4 _array_index_2) SlotNames
        (Utilities|FlowControl|Sequence
          (:then_0
            (for _array_element_5 _skeletalmesh
              (Rendering|Material|SetMaterialbyName _array_element_5 (Utilities|String|StringToName (select RandomizeParameters (Utilities|Array|Get(acopy) SlotNames _array_index) _array_element_4)) (select RandomizeParameters _returnvalue (Utilities|Array|Get(acopy) Materials _array_index_2))))))))))

(event Custom|MoveTo
  (bind _self self)
  (bind _returnvalue (AI|GetAIController _self))
  ;[0.1927 0 0.01304] Basic AI Logic
  (Utilities|FlowControl|Delay (Math|Random|RandomFloatinRange 0.0 3.0))
  (if (Variables|Default|GetChase)
    (AI|AIMoveTo _returnvalue "0, 0, 0" (Game|GetPlayerCharacter 0) -1.0 "Default" "Default" true true
      (:then
        (Utilities|FlowControl|DoOnce false) ; enters at Reset
      ))
    (else
      (AI|Navigation|MovetoLocation _returnvalue (.RandomLocation (AI|Navigation|GetRandomReachablePointinRadius (Transformation|GetActorLocation) 1e+03 0 0)) 2.5e+02 true true false true 0)
      (Utilities|FlowControl|DoOnce false) ; enters at Reset
    )))

(event EventTick
  (params (DeltaSeconds :type Float%20%28single-precision%29))
  ;[0.1927 0 0.01304] Basic AI Logic
  (if (Utilities|Operators|EqualEqual :A (Pawn|Components|CharacterMovement|GetLastUpdateVelocity (Variables|Character|GetCharacterMovement)))
    (Utilities|FlowControl|DoOnce false
      (:Completed
        (CallFunction|Moveto)))))

(event EventBeginPlay
  ;[0.05725 1 0] Initialize - Random Movement Speed + Random Outfit on Begin Play
  (Variables|/Script/Engine.CharacterMovementComponent|SetMaxWalkSpeed (Variables|Character|GetCharacterMovement) (Math|Random|RandomFloatinRange (Variables|Default|GetMinWalkSpeed) (Variables|Default|GetMaxWalkSpeed)))
  ;;[0.009027 0 1] Set to your own Character Controller
  (bind _output_get (Variables|Default|SetAs%20BPC%20Outfit%20Controller (Actor|GetComponentbyClass "/Game/YI_ModularZombies/Blueprints/Master/Components/BPC_OutfitController.BPC_OutfitController_C")))
  (Utilities|IsValid _output_get
    (:Is%20Valid
      (if (Variables|/Game/YI_ModularZombies/Blueprints/Master/Components/BPC_OutfitController.BPC_OutfitController_C|GetRandomizeOnBeginPlay _output_get)
        (Default|RandomizeSelected _output_get)))))

(fn ConstructionScript
  (bind _output_get (Variables|Default|SetAs%20BPC%20Outfit%20Controller (Actor|GetComponentbyClass "/Game/YI_ModularZombies/Blueprints/Master/Components/BPC_OutfitController.BPC_OutfitController_C")))
  (Default|RandomizeSelected _output_get))