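; Data object for an entry in an interactable computer's list, handling what happens when that entry's button is pressed.
; An exit entry returns the view to the player camera.
; Other entries switch the computer widget to show their title and text, play any attached media on the interacted computer, and open any linked door.
; When the video ends, the widget switches back to the menu.
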(event Custom|Button%20Pressed
  (bind _data (Variables|Default|GetData))
  (if (Variables|Default|GetExitComputer)
    (bind _player_character (Variables|Default|GetPlayer%20Character)
      (:then
        (Class|PlayerCharacter|SwitchBacktoPlayerCamera _player_character))
      (:else))
    (else
      (Utilities|FlowControl|Sequence
        (:then_0
          (bind _computer_widget (Variables|Default|GetComputer%20Widget)
            (:then
              (Default|SwitchtoData _computer_widget (.label _data) (.textdata _data))
              (Utilities|IsValid (.media _data)
                (:Is%20Valid
                  (bind _player_character_2 (Variables|Default|GetPlayer%20Character)
                    (:then
                      (bind _asinteractable_computer (Utilities|Casting|CastToInteractableComputer (Variables|/Script/GAD222.PlayerInteraction|GetInteractable (Variables|/Script/GAD222.PlayerCharacter|GetPlayerInteraction _player_character_2))))
                      (Class|InteractableComputer|PlayVideo _asinteractable_computer (.media _data))
                      (bind _output_get (Variables|Default|SetMedia%20Player (Variables|/Script/GAD222.InteractableComputer|GetMediaPlayer _asinteractable_computer)))
                      (Media|MediaPlayer|BindEventtoOnEndReached _output_get (delegate Custom|Video%20Finished%20Playing)))
                    (:else)))))
            (:else)))
        (:then_1
          (Utilities|IsValid (.door _data)
            (:Is%20Valid
              (Class|Door|OpenDoor (.door _data)))))))))

(event Custom|Video%20Finished%20Playing
  (bind _computer_widget (Variables|Default|GetComputer%20Widget)
    (:then
      (Default|SwitchtoMenu _computer_widget))
    (:else)))