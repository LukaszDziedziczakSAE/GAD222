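; BP_CinematicCharacter is a character for cinematics that shows either the male (Mike) or female (Maria) player model with matching hair.
; On BeginPlay it reads the MaleCharacter flag from BP_ZombieGameInstance and sets the skeletal mesh assets for body and hair.
; The construction script makes the hair follow the body mesh through a leader pose component, so both animate together.
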(event EventBeginPlay
  (bind _asbp_zombie_game_instance (Utilities|Casting|CastToBP_ZombieGameInstance (Game|GetGameInstance)))
  (if (Variables|/Script/GAD222.ZombieGameInstance|GetbMaleCharacter _asbp_zombie_game_instance)
    (Components|SkeletalMesh|SetSkeletalMeshAsset (Variables|Character|GetMesh) (Variables|Default|GetMike))
    (Components|SkeletalMesh|SetSkeletalMeshAsset (Variables|Default|GetHair) (Variables|Default|GetMike%20Hair))
    (else
      (Components|SkeletalMesh|SetSkeletalMeshAsset (Variables|Character|GetMesh) (Variables|Default|GetMaria))
      (Components|SkeletalMesh|SetSkeletalMeshAsset (Variables|Default|GetHair) (Variables|Default|GetMaria%20Hair)))))

(fn ConstructionScript
  (Components|SkinnedMesh|SetLeaderPoseComponent (Variables|Default|GetHair) (Variables|Character|GetMesh) false false))